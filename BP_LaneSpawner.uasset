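; Lane spawner that builds a chunk of terrain for a chicken-crossing game and chains to another spawner as the player advances.
; BeginPlay lays a row of actors along X from its mesh: grass first, then random picks, with some branches lacking a class.
; A fixed lane partway along also gets a TriggerZone.
; When ChickenCharacter overlaps it, a DoOnce computes the next chunk's location and spawns another BP_LaneSpawner, without passing that location.
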(event Custom|OnActorBeginOverlap_Event_0
  (params (OverlappedActor :type Actor%20Object%20Reference) (OtherActor :type Actor%20Object%20Reference))
  (bind _staticmesh (Variables|Default|GetStaticMesh))
  (bind _returnvalue (Transformation|GetWorldLocation _staticmesh))
  (Utilities|Casting|CastToChickenCharacter OtherActor)
  (Utilities|FlowControl|DoOnce false
    (:Completed
      (Variables|Default|SetSpawnlocation (Math|Vector|MakeVector (+ (.x _returnvalue) 3.1e+03) (.y _returnvalue) (.z _returnvalue)))
      (Game|SpawnActorfromClass "BP_LaneSpawner_C" (Math|Transform|MakeTransform "0, 0, 0" "0, 0, 0" "1.000000,1.000000,1.000000") "Undefined" 0 0))))

(event EventBeginPlay
  (bind _staticmesh (Variables|Default|GetStaticMesh))
  (bind _returnvalue (Transformation|GetWorldLocation _staticmesh))
  (for _index (range 0 30)
    (Variables|Default|SetSpawnlocation (Math|Vector|MakeVector (+ (* _index 100) (.x _returnvalue)) (.y _returnvalue) (.z _returnvalue)))
    (if (Math|Integer|InRange(Integer) _index 0 2)
      (Game|SpawnActorfromClass "/Game/ThirdPerson/Blueprints/grass.grass_C" (Math|Transform|MakeTransform (Variables|Default|GetSpawnlocation) "0, 0, 0" "1.000000,1.000000,1.000000") "Undefined" 0 0)
      (elif (Math|Integer|InRange(Integer) _index 3 9)
        (switch int (Math|Random|RandomIntegerinRange 0 3) :!label _label
          (:0
            (Game|SpawnActorfromClass "/Game/ThirdPerson/Blueprints/lane.lane_C" (Math|Transform|MakeTransform (Variables|Default|GetSpawnlocation) "0, 0, 0" "1.000000,1.000000,1.000000") "Undefined" 0 0))
          (:1
            (Game|SpawnActorfromClass "/Game/ThirdPerson/Blueprints/lane.lane_C" (Math|Transform|MakeTransform (Variables|Default|GetSpawnlocation) "0, 0, 0" "1.000000,1.000000,1.000000") "Undefined" 0 0))
          (:2
            (Game|SpawnActorfromClass "/Game/ThirdPerson/Blueprints/lane.lane_C" (Math|Transform|MakeTransform (Variables|Default|GetSpawnlocation) "0, 0, 0" "1.000000,1.000000,1.000000") "Undefined" 0 0))
          (:3
            (Game|SpawnActorfromClass "/Game/ThirdPerson/Blueprints/grass.grass_C" (Math|Transform|MakeTransform (Variables|Default|GetSpawnlocation) "0, 0, 0" "1.000000,1.000000,1.000000") "Undefined" 0 0)))
        (elif (== _index 10)
          (Game|SpawnActorfromClass "/Game/ThirdPerson/Blueprints/lane.lane_C" (Math|Transform|MakeTransform (Variables|Default|GetSpawnlocation) "0, 0, 0" "1.000000,1.000000,1.000000") "Undefined" 0 0)
          (bind _returnvalue_2 (Game|SpawnActorfromClass "/Game/ThirdPerson/Blueprints/TriggerZone.TriggerZone_C" (Math|Transform|MakeTransform (Variables|Default|GetSpawnlocation) "0, 0, 0" "1.000000,1.000000,1.000000") "Undefined" 0 0))
          (EventDispatchers|AssignOnActorBeginOverlap _returnvalue_2 (delegate Custom|OnActorBeginOverlap_Event_0))
          (elif (Math|Integer|InRange(Integer) _index 10 30)
            (goto _label)))))))

(event Collision|EventActorBeginOverlap
  (params (OtherActor :type Actor%20Object%20Reference)))

(event EventTick
  (params (DeltaSeconds :type Float%20%28single-precision%29)))

(fn ConstructionScript)

(fn SpawnLane
  (params (SpawnLocation :type Vector))
  (bind _returnvalue (Game|SpawnActorfromClass "/Game/ThirdPerson/Blueprints/lane.lane_C" (Math|Transform|MakeTransform SpawnLocation "0, 0, 0" "1.000000,1.000000,1.000000") "Undefined" 0 0))
  (Variables|Default|SetNewestLane _returnvalue))

(fn SpawnLaneatSpawnPoint)